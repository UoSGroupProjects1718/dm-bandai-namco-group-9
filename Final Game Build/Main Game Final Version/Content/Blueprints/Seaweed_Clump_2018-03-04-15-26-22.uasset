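; Seaweed clump actor: a placeholder sprite that fades in on spawn and drifts horizontally across the screen.
; The construction script creates a dynamic material instance, whose Opacity_Level starts at zero on BeginPlay and rises every Tick by the Fadein rate.
; Tick also moves the actor along X at MovementSpeed, like the torpedoes, and destroys it once it passes either off-screen X limit.
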(event EventBeginPlay
  ;[1 1 1] Sets the seaweed to be invisible upon spawn
  (Rendering|Material|SetScalarParameterValue (Variables|Default|GetDynamic_Material_Seaweed) "Opacity_Level" 0.0 :!class /Script/Engine.MaterialInstanceDynamic)
  (Development|PrintString "Seaweed Spawned"))

(event Collision|EventActorBeginOverlap
  (params (OtherActor :type Actor%20Object%20Reference)))

(event EventTick
  (params (DeltaSeconds :type Float%20%28single-precision%29))
  (bind _returnvalue (Transformation|GetActorLocation))
  (bind _dynamic_material_seaweed (Variables|Default|GetDynamic_Material_Seaweed))
  (bind (_x _y _z) (Math|Vector|BreakVector _returnvalue))
  ;[1 1 1] Fades the sprite back into visibility upon spawning
  (bind _returnvalue_2 (Rendering|Material|GetScalarParameterValue _dynamic_material_seaweed "Opacity_Level" :!class /Script/Engine.MaterialInstanceDynamic))
  (Rendering|Material|SetScalarParameterValue _dynamic_material_seaweed "Opacity_Level" (+ _returnvalue_2 (* (Variables|Default|GetFadein) DeltaSeconds)) :!class /Script/Engine.MaterialInstanceDynamic)
  ;[1 1 1] Handles movement. Effectively identical to the code used for the movement of the torpedoes.
  (Transformation|SetActorLocation (Math|Vector|MakeVector (+ (* DeltaSeconds (Variables|Default|GetMovement%20Speed)) _x) _y _z) false false)
  ;[1 1 1] Destroys the seaweed if it gets off scrren
  (if (<= _x -6e+02)
    (Development|PrintString "Seaweed off screen, deleting" :!label _label)
    (Actor|DestroyActor)
    (elif (>= _x 1.4e+03)
      (goto _label))))

(fn ConstructionScript
  (bind _returnvalue (Rendering|Material|CreateDynamicMaterialInstance (Variables|Default|GetSeaweed_Placeholder_Sprite) 0 0 :!class /Script/Engine.PrimitiveComponent))
  (Variables|Default|SetDynamic_Material_Seaweed _returnvalue))