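; Destroyer obstacle that travels along the X axis and drops depth charges meant to land on players below.
; Tick advances X by MovementSpeed and spawns an Obstacle_Depth_Charge near either of two hardcoded X positions, intended as player locations.
; A DroppingMine flag with a one-second Delay prevents repeat drops.
; Off-screen cleanup is a 40-second Delay started from Tick before DestroyActor, with no actual position check.
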(event EventBeginPlay)

(event Collision|EventActorBeginOverlap
  (params (OtherActor :type Actor%20Object%20Reference)))

(event EventTick
  (params (DeltaSeconds :type Float%20%28single-precision%29))
  (bind _returnvalue (Transformation|GetActorLocation))
  (bind (_x _y _z) (Math|Vector|BreakVector _returnvalue))
  ;[1 1 1] Handles movement. Effectively identical to the code used for the movement of the torpedoes.
  (Transformation|SetActorLocation (Math|Vector|MakeVector (+ (* DeltaSeconds (Variables|Default|GetMovement_Speed)) _x) _y _z) false false)
  ;[1 1 1] Spawns Depth Charges directly above players, dropping one every time it passes a player's location
  (if (not (Variables|Default|GetDropping_Mine))
    (if (Math|Float|NearlyEqual(Float) _x 0.0 1.0)
      (Variables|Default|SetDropping_Mine true :!label _label)
      (Game|SpawnActorfromClass "/Game/Blueprints/Obstacle_Depth_Charge.Obstacle_Depth_Charge_C" (Transformation|GetActorTransform) "Undefined" 0 0)
      (Utilities|FlowControl|Delay 1.0)
      (Variables|Default|SetDropping_Mine false)
      (elif (Math|Float|NearlyEqual(Float) _x 8e+02 1.0)
        (goto _label)
        (else
          ;[1 1 1] Destroys the Destroyer if it gets off scrren
          (Utilities|FlowControl|Delay 4e+01)
          (Development|PrintString "Destroyer off screen, destroying")
          (Actor|DestroyActor))))))

(fn ConstructionScript)