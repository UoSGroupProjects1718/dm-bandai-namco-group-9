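; Underwater mine obstacle that drifts along the X axis and explodes when it touches a player submarine.
; The construction script makes a dynamic material on the sprite; BeginPlay zeroes its opacity and Tick fades it in while moving the mine.
; Leaving the horizontal bounds destroys it with an explosion emitter.
; Overlap with any listed P1/P2 submarine class triggers a brief delay, explosion, blast sound and destruction.
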(event EventBeginPlay
  ;[1 1 1] Sets the Mine to be invisible upon spawn
  (Rendering|Material|SetScalarParameterValue (Variables|Default|GetDynamic_Material_Mine) "Opacity_Level" 0.0 :!class /Script/Engine.MaterialInstanceDynamic)
  (Development|PrintString "Mine Spawned"))

(event Collision|EventActorBeginOverlap
  (params (OtherActor :type Actor%20Object%20Reference))
  (bind _returnvalue (Utilities|GetClass OtherActor))
  ;[1 1 1] Destroys the mine after collision with the player's submarine
  (if (or (Math|Boolean|ORBoolean (Utilities|ClassIsChildOf _returnvalue "/Game/Blueprints/P1_Sub_JPN_Easy.P1_Sub_JPN_Easy_C") (Utilities|ClassIsChildOf _returnvalue "/Game/Blueprints/P2_Sub_JPN_Easy.P2_Sub_JPN_Easy_C") (Utilities|ClassIsChildOf _returnvalue "/Game/Blueprints/P1_Sub_JPN_Medium.P1_Sub_JPN_Medium_C") (Utilities|ClassIsChildOf _returnvalue "/Game/Blueprints/P2_Sub_JPN_Medium.P2_Sub_JPN_Medium_C") (Utilities|ClassIsChildOf _returnvalue "/Game/Blueprints/P1_Sub_JPN_Expert.P1_Sub_JPN_Expert_C") (Utilities|ClassIsChildOf _returnvalue "/Game/Blueprints/P2_Sub_JPN_Expert.P2_Sub_JPN_Expert_C") (Utilities|ClassIsChildOf _returnvalue "/Game/Blueprints/P1_Sub_RUS_Easy.P1_Sub_RUS_Easy_C") (Utilities|ClassIsChildOf _returnvalue "/Game/Blueprints/P2_Sub_RUS_Easy.P2_Sub_RUS_Easy_C") (Utilities|ClassIsChildOf _returnvalue "/Game/Blueprints/P1_Sub_RUS_Medium.P1_Sub_RUS_Medium_C") (Utilities|ClassIsChildOf _returnvalue "/Game/Blueprints/P2_Sub_RUS_Medium.P2_Sub_RUS_Medium_C") (Utilities|ClassIsChildOf _returnvalue "/Game/Blueprints/P1_Sub_RUS_Expert.P1_Sub_RUS_Expert_C") (Utilities|ClassIsChildOf _returnvalue "/Game/Blueprints/P2_Sub_RUS_Expert.P2_Sub_RUS_Expert_C") (Utilities|ClassIsChildOf _returnvalue "/Game/Blueprints/P1_Sub_TUR_Easy.P1_Sub_TUR_Easy_C") (Utilities|ClassIsChildOf _returnvalue "/Game/Blueprints/P2_Sub_TUR_Easy.P2_Sub_TUR_Easy_C") (Utilities|ClassIsChildOf _returnvalue "/Game/Blueprints/P1_Sub_TUR_Medium.P1_Sub_TUR_Medium_C") (Utilities|ClassIsChildOf _returnvalue "/Game/Blueprints/P2_Sub_TUR_Medium.P2_Sub_TUR_Medium_C") (Utilities|ClassIsChildOf _returnvalue "/Game/Blueprints/P1_Sub_TUR_Expert.P1_Sub_TUR_Expert_C") (Utilities|ClassIsChildOf _returnvalue "/Game/Blueprints/P2_Sub_TUR_Expert.P2_Sub_TUR_Expert_C") (Utilities|ClassIsChildOf _returnvalue "/Game/Blueprints/P1_Sub_ENG_Easy.P1_Sub_ENG_Easy_C") (Utilities|ClassIsChildOf _returnvalue "/Game/Blueprints/P2_Sub_ENG_Easy.P2_Sub_ENG_Easy_C") (Utilities|ClassIsChildOf _returnvalue "/Game/Blueprints/P1_Sub_ENG_Medium.P1_Sub_ENG_Medium_C") (Utilities|ClassIsChildOf _returnvalue "/Game/Blueprints/P2_Sub_ENG_Medium.P2_Sub_ENG_Medium_C") (Utilities|ClassIsChildOf _returnvalue "/Game/Blueprints/P1_Sub_ENG_Expert.P1_Sub_ENG_Expert_C") (Utilities|ClassIsChildOf _returnvalue "/Game/Blueprints/P2_Sub_ENG_Expert.P2_Sub_ENG_Expert_C") (Utilities|ClassIsChildOf _returnvalue "/Game/Blueprints/P1_Sub_USA_Easy.P1_Sub_USA_Easy_C")) (Math|Boolean|ORBoolean (Utilities|ClassIsChildOf _returnvalue "/Game/Blueprints/P2_Sub_USA_Easy.P2_Sub_USA_Easy_C") (Utilities|ClassIsChildOf _returnvalue "/Game/Blueprints/P1_Sub_USA_Medium.P1_Sub_USA_Medium_C") (Utilities|ClassIsChildOf _returnvalue "/Game/Blueprints/P2_Sub_USA_Medium.P2_Sub_USA_Medium_C") (Utilities|ClassIsChildOf _returnvalue "/Game/Blueprints/P1_Sub_USA_Expert.P1_Sub_USA_Expert_C") (Utilities|ClassIsChildOf _returnvalue "/Game/Blueprints/P2_Sub_USA_Expert.P2_Sub_USA_Expert_C")))
    (Utilities|FlowControl|Delay 0.1)
    (Effects|SpawnEmitteratLocation "/Game/Particles/Underwater_Explosion.Underwater_Explosion" (Transformation|GetActorLocation))
    (Audio|SpawnSound2D "/Game/Audio/Depth_Charge_Blast.Depth_Charge_Blast")
    (Actor|DestroyActor)))

(event EventTick
  (params (DeltaSeconds :type Float%20%28single-precision%29))
  (bind _returnvalue (Transformation|GetActorLocation))
  (bind _dynamic_material_mine (Variables|Default|GetDynamic_Material_Mine))
  (bind (_x _y _z) (Math|Vector|BreakVector _returnvalue))
  ;[1 1 1] Fades the sprite back into visibility upon spawning
  (bind _returnvalue_2 (Rendering|Material|GetScalarParameterValue _dynamic_material_mine "Opacity_Level" :!class /Script/Engine.MaterialInstanceDynamic))
  (Rendering|Material|SetScalarParameterValue _dynamic_material_mine "Opacity_Level" (+ _returnvalue_2 (* (Variables|Default|GetFadein) DeltaSeconds)) :!class /Script/Engine.MaterialInstanceDynamic)
  ;[1 1 1] Handles movement. Effectively identical to the code used for the movement of the torpedoes.
  (Transformation|SetActorLocation (Math|Vector|MakeVector (+ (* DeltaSeconds (Variables|Default|GetMovement%20Speed)) _x) _y _z) false false)
  ;[1 1 1] Destroys the mine if it gets off scrren
  (if (<= _x -6e+02)
    (Development|PrintString "Mine off screen, deleting" :!label _label)
    (Effects|SpawnEmitteratLocation "/Game/Particles/Underwater_Explosion.Underwater_Explosion" (Transformation|GetActorLocation))
    (Actor|DestroyActor)
    (elif (>= _x 1.4e+03)
      (goto _label))))

(fn ConstructionScript
  (bind _returnvalue (Rendering|Material|CreateDynamicMaterialInstance (Variables|Default|GetUnderwater_Mine_Sprite) 0 0 :!class /Script/Engine.PrimitiveComponent))
  (Variables|Default|SetDynamic_Material_Mine _returnvalue))