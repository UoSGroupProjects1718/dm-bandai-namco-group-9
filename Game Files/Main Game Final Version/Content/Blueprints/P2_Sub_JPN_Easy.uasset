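; Player 2's Japanese submarine, which dives, fires torpedoes and takes damage from enemy torpedoes and obstacles.
; Holding Down sinks it to a depth limit; releasing fires a cooldown-gated torpedo and lets Tick float it back up.
; Overlaps subtract hull integrity, flag boulder damage over time or halve speed in seaweed.
; Tick swaps damage sprites by hull level, and a shared death check opens the paused Game Over screen.
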(event EventBeginPlay
  ;[1 1 1] Allows the player to control the sub.
  (Input|EnableInput (Game|GetPlayerController 0)))

(event Collision|EventActorEndOverlap
  (params (OtherActor :type Actor%20Object%20Reference))
  ;[1 1 1] Checks if the player is caught in seaweed. If so, cuts the movement of the sub in half. Upon leaving, doubles the speed returning the sub to maximum.
  (if (Utilities|ClassIsChildOf (Utilities|GetClass OtherActor) "/Game/Blueprints/Seaweed_Clump_2018-03-04-15-26-22.Seaweed_Clump_C")
    (Development|PrintString "Player 2 has left the seaweed, speed restored")
    (Variables|Default|SetMovement_Speed (* (Variables|Default|GetMovement_Speed) 2.0))
    (else
      ;[1 1 1] Handles collision with boulders
      (Variables|Default|SetBoulder_Collision false))))

(event EventTick
  (params (DeltaSeconds :type Float%20%28single-precision%29))
  (bind _returnvalue (Transformation|GetActorLocation))
  (bind _returnvalue_2 (Game|GetPlayerController 0))
  (bind _japanese_basic_sub_sprite (Variables|Default|GetJapanese_basic_sub_Sprite))
  (bind _movement_speed (Variables|Default|GetMovement_Speed))
  (bind (_x _y _z) (Math|Vector|BreakVector _returnvalue))
  (bind _returnvalue_3 (* _movement_speed -1.0))
  (bind _returnvalue_4 (* _returnvalue_3 DeltaSeconds))
  (bind _returnvalue_5 (+ _z _returnvalue_4))
  ;[1 1 1] Handles the switching of Sprites when the sub has taken damage
  (if (and (<= (Variables|Default|GetHull_Integrity_P2) 0.75) (>= (Variables|Default|GetHull_Integrity_P2) 0.5))
    (Rendering|Components|Sprite|SetSprite _japanese_basic_sub_sprite "/Game/Art/Subs/Damaged/Japanese_stage_1_75__health_sub_Sprite.Japanese_stage_1_75__health_sub_Sprite"))
  (if (and (<= (Variables|Default|GetHull_Integrity_P2) 0.49) (>= (Variables|Default|GetHull_Integrity_P2) 0.25))
    (Rendering|Components|Sprite|SetSprite _japanese_basic_sub_sprite "/Game/Art/Subs/Damaged/Japanese_stage_1_50__health_sub_Sprite.Japanese_stage_1_50__health_sub_Sprite"))
  (if (and (<= (Variables|Default|GetHull_Integrity_P2) 0.24) (>= (Variables|Default|GetHull_Integrity_P2) 0.01))
    (Rendering|Components|Sprite|SetSprite _japanese_basic_sub_sprite "/Game/Art/Subs/Damaged/Japanese_stage_1_25__health_sub_Sprite.Japanese_stage_1_25__health_sub_Sprite"))
  (if (== (Variables|Default|GetHull_Integrity_P2) 0.0)
    (Rendering|Components|Sprite|SetSprite _japanese_basic_sub_sprite "/Game/Art/Subs/Damaged/Japanese_stage_1_destroyed_sub_Sprite.Japanese_stage_1_destroyed_sub_Sprite"))
  ;[1 1 1] This section controls the submarine's movement. If the sub is already at the surface, or reaches the seafloor it will stop moving. If the player does not tell it to submerge, it will automatically return to to the surface
  (if (Variables|Default|GetP1_Pressed)
    (if (> _returnvalue_5 -3e+02)
      (Transformation|SetActorLocation (Math|Vector|MakeVector _x _y _returnvalue_5) false false))
    (elif (<= _z 0.0)
      (Transformation|SetActorLocation (Math|Vector|MakeVector _x _y (+ _z (* DeltaSeconds (Variables|Default|GetMovement_Speed)))) false false)))
  ;[1 1 1] Handles the damage over time caused by the boulder obstacle
  (if (Variables|Default|GetBoulder_Collision)
    (Variables|Default|SetHull_Integrity_P2 (+ (Variables|Default|GetHull_Integrity_P2) (* -0.4 DeltaSeconds)))
    ;[1 1 1] Checks if the player was hit by an enemy torpedo (And applies damage dependant on which type it was)
    (if (<= (stale Collision|EventActorBeginOverlap _output_get) 0.0)
      (Utilities|FlowControl|DoOnce false
        (:Completed
          ;[1 1 1] Loads the appropriate Game Over screen when the player dies.
          (Audio|PlaySound2D "/Game/Audio/Sub_Death_Explosion.Sub_Death_Explosion")
          (Utilities|FlowControl|Delay 1.0)
          (bind _returnvalue_6 (UserInterface|CreateWidget "/Game/HUD/Game_Over_P2.Game_Over_P2_C"))
          (UserInterface|Viewport|AddtoViewport _returnvalue_6 0)
          (Input|SetInputModeUIOnly _returnvalue_2 _returnvalue_6 "DoNotLock")
          (Game|SetGamePaused true)
          (Variables|/Script/Engine.PlayerController|SetbShowMouseCursor _returnvalue_2 true))))))

(event Collision|EventActorBeginOverlap
  (params (OtherActor :type Actor%20Object%20Reference))
  (bind _returnvalue (Game|GetPlayerController 0))
  ;[1 1 1] Checks if the player was hit by an enemy torpedo (And applies damage dependant on which type it was)
  (if (Utilities|ClassIsChildOf (Utilities|GetClass OtherActor) "/Game/Blueprints/P1_Conventional_Torpedo.P1_Conventional_Torpedo_C")
    (Development|PrintString "Player 2 has been hit (Conventional Torpedo)")
    (bind _output_get (Variables|Default|SetHull_Integrity_P2 (- (Variables|Default|GetHull_Integrity_P2) 0.2)))
    (Development|PrintString (Utilities|String|ToString(Float) _output_get) :!label _label)
    (if (<= _output_get 0.0)
      (Utilities|FlowControl|DoOnce false
        (:Completed
          ;[1 1 1] Loads the appropriate Game Over screen when the player dies.
          (Audio|PlaySound2D "/Game/Audio/Sub_Death_Explosion.Sub_Death_Explosion")
          (Utilities|FlowControl|Delay 1.0)
          (bind _returnvalue_2 (UserInterface|CreateWidget "/Game/HUD/Game_Over_P2.Game_Over_P2_C"))
          (UserInterface|Viewport|AddtoViewport _returnvalue_2 0)
          (Input|SetInputModeUIOnly _returnvalue _returnvalue_2 "DoNotLock")
          (Game|SetGamePaused true)
          (Variables|/Script/Engine.PlayerController|SetbShowMouseCursor _returnvalue true))))
    (else
      ;[1 1 1] Checks if the player is caught in seaweed. If so, cuts the movement of the sub in half. Upon leaving, doubles the speed returning the sub to maximum.
      (if (Utilities|ClassIsChildOf (Utilities|GetClass OtherActor) "/Game/Blueprints/Seaweed_Clump_2018-03-04-15-26-22.Seaweed_Clump_C")
        (Development|PrintString "Player 2 caught in seaweed, speed reduced")
        (Variables|Default|SetMovement_Speed (/ (Variables|Default|GetMovement_Speed) 2.0))
        (else
          ;[1 1 1] Handles collision with mines
          (if (Utilities|ClassIsChildOf (Utilities|GetClass OtherActor) "/Game/Blueprints/Obstacle_Mine.Obstacle_Mine_C")
            (Development|PrintString "Player 2 has been hit (Naval Mine)")
            (Variables|Default|SetHull_Integrity_P2 (- (Variables|Default|GetHull_Integrity_P2) 0.5))
            (goto _label)
            (else
              ;[1 1 1] Handles collision with Depth Charges
              (if (Utilities|ClassIsChildOf (Utilities|GetClass OtherActor) "/Game/Blueprints/Obstacle_Depth_Charge.Obstacle_Depth_Charge_C")
                (Development|PrintString "Player 2 has been hit (Depth Charge)")
                (Variables|Default|SetHull_Integrity_P2 (- (Variables|Default|GetHull_Integrity_P2) 0.15))
                (goto _label)
                (else
                  ;[1 1 1] Handles collision with boulders
                  (if (Utilities|ClassIsChildOf (Utilities|GetClass OtherActor) "/Game/Blueprints/Obstacle_Boulders.Obstacle_Boulders_C")
                    (Variables|Default|SetBoulder_Collision true)))))))))))

(event Input|KeyboardEvents|Down
  (params (Key :type Key%20Structure))
  (bind _returnvalue (Transformation|GetActorTransform))
  (bind (_location _rotation) (Math|Transform|BreakTransform _returnvalue))
  ;[1 1 1] This section controls the submarine's movement. If the sub is already at the surface, or reaches the seafloor it will stop moving. If the player does not tell it to submerge, it will automatically return to to the surface
  (:Pressed
    (Variables|Default|SetP1_Pressed true))
  (:Released
    (Variables|Default|SetP1_Pressed false)
    ;[1 1 1] Controls firing. Initially, checks if it can fire. If so, it spawns a torpedo at the sub's location, then sets 'Can fire' to false. Untill the firing delay has passed, the ship cannot fire again. Once it has passed, it sets 'Can Fire' back to true.
    (if (Variables|Default|GetCan_Fire)
      (Game|SpawnActorfromClass "/Game/Blueprints/P2_Conventional_Torpedo.P2_Conventional_Torpedo_C" (Math|Transform|MakeTransform _location _rotation "-1.000000,1,1") "Undefined" 0 0)
      (Audio|SpawnSound2D "/Game/Audio/Torpedo_Launch.Torpedo_Launch")
      (Variables|Default|SetCan_Fire false)
      (Utilities|FlowControl|Delay (Variables|Default|GetFiring_Delay))
      (Variables|Default|SetCan_Fire true)
      (Development|PrintString "Reloaded (P2)")
      (else
        (Development|PrintString "Cannot Fire, Reloading")))))

(fn ConstructionScript)