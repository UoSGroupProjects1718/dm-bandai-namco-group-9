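; Depth charge obstacle that fades in on spawn, sinks, and explodes at a random depth or on contact with either player's submarine.
; Construction creates a dynamic sprite material whose opacity BeginPlay zeroes and Tick raises.
; Tick also moves the actor vertically by SinkRate without sweep, detonating once it drops below BlastDepth.
; Overlap with either submarine class triggers a briefly delayed explosion and destroy, applying no damage here.
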(event Collision|EventActorBeginOverlap
  (params (OtherActor :type Actor%20Object%20Reference))
  ;[1 1 1] Destroys the mine after collision with the player's submarine
  (if (Utilities|ClassIsChildOf (Utilities|GetClass OtherActor) "/Game/Blueprints/P1_Sub_JPN_Easy.P1_Sub_JPN_Easy_C")
    (Utilities|FlowControl|Delay 0.1 :!label _label)
    (Effects|SpawnEmitteratLocation "/Game/Particles/Generic_Explosion.Generic_Explosion" (Transformation|GetActorLocation))
    (Actor|DestroyActor)
    (elif (Utilities|ClassIsChildOf (Utilities|GetClass OtherActor) "/Game/Blueprints/P2_Sub_JPN_Easy.P2_Sub_JPN_Easy_C")
      (goto _label))))

(event EventTick
  (params (DeltaSeconds :type Float%20%28single-precision%29))
  (bind _returnvalue (Transformation|GetActorLocation))
  (bind _dynamic_material_depth_charge (Variables|Default|GetDynamic_Material_Depth_Charge))
  (bind (_x _y _z) (Math|Vector|BreakVector _returnvalue))
  ;[1 1 1] Fades the sprite back into visibility upon spawning
  (bind _returnvalue_2 (Rendering|Material|GetScalarParameterValue _dynamic_material_depth_charge "Opacity_Level" :!class /Script/Engine.MaterialInstanceDynamic))
  (Rendering|Material|SetScalarParameterValue _dynamic_material_depth_charge "Opacity_Level" (+ _returnvalue_2 (* (Variables|Default|GetFadein) DeltaSeconds)) :!class /Script/Engine.MaterialInstanceDynamic)
  ;[1 1 1] Handles movement. Effectively identical to the code used for the movement of the torpedoes.
  (Transformation|SetActorLocation (Math|Vector|MakeVector _x _y (+ (* DeltaSeconds (Variables|Default|GetSink_Rate)) _z)) false false)
  ;[1 1 1] Detonates the charge at the predetermed depth
  (if (< _z (Variables|Default|GetBlast_Depth))
    (Development|PrintString "Depth Charge Detonated")
    (Effects|SpawnEmitteratLocation "/Game/Particles/Generic_Explosion.Generic_Explosion" (Transformation|GetActorLocation))
    (Actor|DestroyActor)))

(event EventBeginPlay
  ;[1 1 1] Sets the Mine to be invisible upon spawn
  (Rendering|Material|SetScalarParameterValue (Variables|Default|GetDynamic_Material_Depth_Charge) "Opacity_Level" 0.0 :!class /Script/Engine.MaterialInstanceDynamic)
  (Development|PrintString "Depth Charge Spawned")
  ;[1 1 1] Sets a random depth for detonation
  (Variables|Default|SetBlast_Depth (Math|Random|RandomFloatinRange -4e+01 -2e+02)))

(fn ConstructionScript
  (bind _returnvalue (Rendering|Material|CreateDynamicMaterialInstance (Variables|Default|GetDepth_Charge_Placeholder_Sprite) 0 0 :!class /Script/Engine.PrimitiveComponent))
  (Variables|Default|SetDynamic_Material_Depth_Charge _returnvalue))