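; Obstacle spawner that periodically creates Seaweed_Clump actors at a fixed X position and random height, moving in alternating directions.
; BeginPlay randomizes the first direction and height and sets a fixed speed and delay.
; Tick uses a Processing flag as a gate around a Delay, forming a repeating spawn loop.
; Each pass offsets the new clump's MovementSpeed by direction, rerolls height and flips direction.
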(event EventBeginPlay
  ;[1 1 1] Sets all values randomly upon loading in.
  (Variables|Default|SetSeaweed_Movement_Direction (Math|Random|RandomBool))
  (Variables|Default|SetSeaweed_Spawn_Height (Math|Random|RandomFloatinRange -3e+02 2e+01))
  (Variables|Default|SetSeaweed_Movement_Speed 6e+01)
  (Variables|Default|SetSeaweed_Spwan_Delay 1e+01))

(event Collision|EventActorBeginOverlap
  (params (OtherActor :type Actor%20Object%20Reference)))

(event EventTick
  (params (DeltaSeconds :type Float%20%28single-precision%29))
  ;[1 1 1] First, checks if it's already proccessing a spawn. If not, it activates proccessing so it won't keep repeatedly spawning. After a (random) delay time, it spawns a seaweed clump at a randomly chosen height, and spawns it. It then gives it a speed value. If 'Seaweed Movement Direction' is true, it'll invert the speed, causing the seaweed to move the other way. It automatically switches direction each time it finishes spawning. Once it's done, processing is set back to false so the whole loop can start again.
  (if (not (Variables|Default|GetProcessing))
    (Variables|Default|SetProcessing true)
    (Utilities|FlowControl|Delay (Variables|Default|GetSeaweed_Spwan_Delay))
    (bind _returnvalue (Game|SpawnActorfromClass "/Game/Blueprints/Seaweed_Clump_2018-03-04-15-26-22.Seaweed_Clump_C" (Math|Transform|MakeTransform (Math|Vector|MakeVector 4e+02 -1.0 (Variables|Default|GetSeaweed_Spawn_Height)) "0, 0, 0" "-1.000000,1,1") "Undefined" 0 0))
    (Transformation|SetActorTransform _returnvalue (Math|Transform|MakeTransform (.Location (Math|Transform|BreakTransform (Transformation|GetActorTransform _returnvalue))) (.Rotation (Math|Transform|BreakTransform (Transformation|GetActorTransform _returnvalue))) (Math|Vector|MakeVector (.X%20Out (|CollapseGraph_0 (.X (Math|Vector|BreakVector (.Scale (Math|Transform|BreakTransform (Transformation|GetActorTransform _returnvalue))))) (.Y (Math|Vector|BreakVector (.Scale (Math|Transform|BreakTransform (Transformation|GetActorTransform _returnvalue))))) (.Z (Math|Vector|BreakVector (.Scale (Math|Transform|BreakTransform (Transformation|GetActorTransform _returnvalue))))))) (.Y%20Out (|CollapseGraph_0 (.X (Math|Vector|BreakVector (.Scale (Math|Transform|BreakTransform (Transformation|GetActorTransform _returnvalue))))) (.Y (Math|Vector|BreakVector (.Scale (Math|Transform|BreakTransform (Transformation|GetActorTransform _returnvalue))))) (.Z (Math|Vector|BreakVector (.Scale (Math|Transform|BreakTransform (Transformation|GetActorTransform _returnvalue))))))) (.Z%20Out (|CollapseGraph_0 (.X (Math|Vector|BreakVector (.Scale (Math|Transform|BreakTransform (Transformation|GetActorTransform _returnvalue))))) (.Y (Math|Vector|BreakVector (.Scale (Math|Transform|BreakTransform (Transformation|GetActorTransform _returnvalue))))) (.Z (Math|Vector|BreakVector (.Scale (Math|Transform|BreakTransform (Transformation|GetActorTransform _returnvalue))))))))))
    (if (Variables|Default|GetSeaweed_Movement_Direction)
      (Variables|/Game/Blueprints/Seaweed_Clump_2018-03-04-15-26-22.Seaweed_Clump_C|SetMovement%20Speed _returnvalue (- (Variables|/Game/Blueprints/Seaweed_Clump_2018-03-04-15-26-22.Seaweed_Clump_C|GetMovement%20Speed _returnvalue) (Variables|Default|GetSeaweed_Movement_Speed)))
      (else
        (Variables|/Game/Blueprints/Seaweed_Clump_2018-03-04-15-26-22.Seaweed_Clump_C|SetMovement%20Speed _returnvalue (+ (Variables|/Game/Blueprints/Seaweed_Clump_2018-03-04-15-26-22.Seaweed_Clump_C|GetMovement%20Speed _returnvalue) (Variables|Default|GetSeaweed_Movement_Speed)))))
    (Variables|Default|SetSeaweed_Spawn_Height (Math|Random|RandomFloatinRange -3e+02 2e+01))
    (Variables|Default|SetSeaweed_Movement_Speed 6e+01)
    (Variables|Default|SetSeaweed_Spwan_Delay 1e+01)
    (Variables|Default|SetSeaweed_Movement_Direction (not (Variables|Default|GetSeaweed_Movement_Direction)))
    (Variables|Default|SetProcessing false)))

(fn ConstructionScript)