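; Player 1's submarine, which dives while S is held and rises toward the surface when released, within fixed depth limits.
; Releasing S also fires a conventional torpedo, gated by a reload delay.
; Overlaps with P2 torpedoes or mines reduce hull integrity, while seaweed halves speed until exit; depth-charge damage is unconnected.
; At zero hull, the game pauses and shows the Game_Over_P2 widget.
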(event EventBeginPlay
  ;[1 1 1] Allows the player to control the sub.
  (Input|EnableInput (Game|GetPlayerController 0)))

(event Collision|EventActorEndOverlap
  (params (OtherActor :type Actor%20Object%20Reference))
  ;[1 1 1] Checks if the player is caught in seaweed. If so, cuts the movement of the sub in half. Upon leaving, doubles the speed returning the sub to maximum.
  (if (Utilities|ClassIsChildOf (Utilities|GetClass OtherActor) "/Game/Blueprints/Seaweed_Clump_2018-03-04-15-26-22.Seaweed_Clump_C")
    (Development|PrintString "Player 1 has left the seaweed, speed restored")
    (Variables|Default|SetMovement_Speed (* (Variables|Default|GetMovement_Speed) 2.0))))

(event EventTick
  (params (DeltaSeconds :type Float%20%28single-precision%29))
  (bind _returnvalue (Transformation|GetActorLocation))
  (bind _movement_speed (Variables|Default|GetMovement_Speed))
  (bind (_x _y _z) (Math|Vector|BreakVector _returnvalue))
  (bind _returnvalue_2 (* _movement_speed -1.0))
  (bind _returnvalue_3 (* _returnvalue_2 DeltaSeconds))
  (bind _returnvalue_4 (+ _z _returnvalue_3))
  ;[1 1 1] This section controls the submarine's movement. If the sub is already at the surface, or reaches the seafloor it will stop moving. If the player does not tell it to submerge, it will automatically return to to the surface
  (if (Variables|Default|GetP1_Pressed)
    (if (> _returnvalue_4 -3e+02)
      (Transformation|SetActorLocation (Math|Vector|MakeVector _x _y _returnvalue_4) false false))
    (elif (<= _z 0.0)
      (Transformation|SetActorLocation (Math|Vector|MakeVector _x _y (+ _z (* DeltaSeconds (Variables|Default|GetMovement_Speed)))) false false))))

(event Collision|EventActorBeginOverlap
  (params (OtherActor :type Actor%20Object%20Reference))
  (bind _returnvalue (Game|GetPlayerController 0))
  ;[1 1 1] Checks if the player was hit by an enemy torpedo and which sort, and takes off some health. If the players health is at 0 or lower after a hit, it destroys them.
  (if (Utilities|ClassIsChildOf (Utilities|GetClass OtherActor) "/Game/Blueprints/P2_Conventional_Torpedo.P2_Conventional_Torpedo_C")
    (Development|PrintString "Player 1 has been hit (Conventional Torpedo)")
    (bind _output_get (Variables|Default|SetHull_Integrity_P1 (- (Variables|Default|GetHull_Integrity_P1) 0.2)))
    (Development|PrintString (Utilities|String|ToString(Float) _output_get) :!label _label)
    (if (<= _output_get 0.0)
      (Development|PrintString "P1 Destroyed")
      (if (<= (Variables|Default|GetHull_Integrity_P1) 0.0)
        (bind _returnvalue_2 (UserInterface|CreateWidget "/Game/HUD/Game_Over_P2.Game_Over_P2_C"))
        (UserInterface|Viewport|AddtoViewport _returnvalue_2 0)
        (Input|SetInputModeUIOnly _returnvalue _returnvalue_2 "DoNotLock")
        (Game|SetGamePaused true)
        (Variables|/Script/Engine.PlayerController|SetbShowMouseCursor _returnvalue true)))
    (else
      ;[1 1 1] Checks if the player is caught in seaweed. If so, cuts the movement of the sub in half. Upon leaving, doubles the speed returning the sub to maximum.
      (if (Utilities|ClassIsChildOf (Utilities|GetClass OtherActor) "/Game/Blueprints/Seaweed_Clump_2018-03-04-15-26-22.Seaweed_Clump_C")
        (Development|PrintString "Player 1caught in seaweed, speed reduced")
        (Variables|Default|SetMovement_Speed (/ (Variables|Default|GetMovement_Speed) 2.0))
        (else
          ;[1 1 1] Handles collision with mines
          (if (Utilities|ClassIsChildOf (Utilities|GetClass OtherActor) "/Game/Blueprints/Obstacle_Mine.Obstacle_Mine_C")
            (Development|PrintString "Player 1 has been hit (Naval Mine)")
            (Variables|Default|SetHull_Integrity_P1 (- (Variables|Default|GetHull_Integrity_P1) 0.5))
            (goto _label)))))))

(event Input|KeyboardEvents|S
  (params (Key :type Key%20Structure))
  (bind _returnvalue (Transformation|GetActorTransform))
  (bind (_location _rotation) (Math|Transform|BreakTransform _returnvalue))
  ;[1 1 1] This section controls the submarine's movement. If the sub is already at the surface, or reaches the seafloor it will stop moving. If the player does not tell it to submerge, it will automatically return to to the surface
  (:Pressed
    (Variables|Default|SetP1_Pressed true))
  (:Released
    (Variables|Default|SetP1_Pressed false)
    ;[1 1 1] Controls firing. Initially, checks if it can fire. If so, it spawns a torpedo at the sub's location, then sets 'Can fire' to false. Untill the firing delay has passed, the ship cannot fire again. Once it has passed, it sets 'Can Fire' back to true.
    (if (Variables|Default|GetCan_Fire)
      (Game|SpawnActorfromClass "/Game/Blueprints/P1_Conventional_Torpedo.P1_Conventional_Torpedo_C" (Math|Transform|MakeTransform _location _rotation) "Undefined" 0 0)
      (Variables|Default|SetCan_Fire false)
      (Utilities|FlowControl|Delay (Variables|Default|GetFiring_Delay))
      (Variables|Default|SetCan_Fire true)
      (Development|PrintString "Reloaded (P1)")
      (else
        (Development|PrintString "Cannot Fire, Reloading")))))

(fn ConstructionScript)