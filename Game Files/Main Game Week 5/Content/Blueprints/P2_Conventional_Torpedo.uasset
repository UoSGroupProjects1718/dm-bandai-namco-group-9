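; Player 2 conventional torpedo actor that explodes on overlapping a P1_Sub_JPN_Easy submarine.
; Tick moves it along world X without sweep, scaled by delta time, and adjusts velocity from SpeedController values when the minimum exceeds the maximum.
; A hit spawns an explosion and destroys the torpedo after a short delay intended to let the target register it.
; BeginPlay starts a timeout that destroys missed torpedoes.
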(event EventTick
  (params (DeltaSeconds :type Float%20%28single-precision%29))
  (bind _returnvalue (Transformation|GetActorLocation))
  (bind (_minimum_torpedo_velocity _torpedo_acceleration _maximum_torpedo_velocity) (|SpeedController))
  (bind (_x _y _z) (Math|Vector|BreakVector _returnvalue))
  ;[1 1 1] Causes the torpedo to automatically move. The torpedo will accelerate to a maxium value set by the relevant floats
  (Transformation|SetActorLocation (Math|Vector|MakeVector (+ _x (* (* (Variables|Default|GetMinimum_Torpedo_Velocity) 1.0) DeltaSeconds)) _y _z) false false)
  (if (> _minimum_torpedo_velocity _maximum_torpedo_velocity)
    (Variables|Default|SetMinimum_Torpedo_Velocity (+ _minimum_torpedo_velocity _torpedo_acceleration))))

(event EventBeginPlay
  ;[1 1 1] Auto-destroys the torpedo should it miss it's target.
  (Utilities|FlowControl|Delay 7.0)
  (Actor|DestroyActor)
  (Development|PrintString "Torpedo Timed out (P2)"))

(event Collision|EventActorBeginOverlap
  (params (OtherActor :type Actor%20Object%20Reference))
  ;[1 1 1] Checks to see if the torpedo has hit it's target, then destroys it after a short delay to ensure it doesn't disapear before the hit was registered at the other end.
  (if (Utilities|ClassIsChildOf (Utilities|GetClass OtherActor) "/Game/Blueprints/P1_Sub_JPN_Easy.P1_Sub_JPN_Easy_C")
    (Effects|SpawnEmitteratLocation "/Game/Particles/Generic_Explosion.Generic_Explosion" (Transformation|GetActorLocation))
    (Development|PrintString "Hit confirmed, destroying torpedo (P2)")
    (Utilities|FlowControl|Delay 0.1)
    (Actor|DestroyActor)))

(fn ConstructionScript)