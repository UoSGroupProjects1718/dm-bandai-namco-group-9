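; Spawner actor that periodically sends pairs of Obstacle_Destroyer ships in from opposite off-screen sides, using a variant of the Mine spawner method.
; Tick runs a Delay, which is set to a minute after the first wave, then spawns both destroyers at a shared height.
; A direction flag flips between spawns to choose start X and speed sign, with the first ship mirrored by negative X scale.
; SpawnCounter resets after each pair, repeating the cycle.
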(event EventBeginPlay)

(event Collision|EventActorBeginOverlap
  (params (OtherActor :type Actor%20Object%20Reference)))

(event EventTick
  (params (DeltaSeconds :type Float%20%28single-precision%29))
  ;[1 1 1] Uses a similar spawning method to the Mine spawner but with a slight modification. The spawn points, being off screen have to be set depending on the direction of movement. Other than that, it is identical.
  (if (< (Variables|Default|GetSpawn%20Counter) 2.0)
    (if (Variables|Default|GetDestroyer_Movement_Direction)
      (Variables|Default|SetDestroyer_Spawn_Point 1.2e+03)
      (else
        (Variables|Default|SetDestroyer_Spawn_Point -4e+02)))
    (Utilities|FlowControl|Delay (Variables|Default|GetDestroyer_Spawn_Delay))
    (bind _returnvalue (Game|SpawnActorfromClass "/Game/Blueprints/Obstacle_Destroyer.Obstacle_Destroyer_C" (Math|Transform|MakeTransform (Math|Vector|MakeVector (Variables|Default|GetDestroyer_Spawn_Point) 0.0 (Variables|Default|GetDestroyer_Spawn_Height)) "0, 0, 0" "-1.000000,1,1") "Undefined" 0 0))
    (if (Variables|Default|GetDestroyer_Movement_Direction)
      (Variables|/Game/Blueprints/Obstacle_Destroyer.Obstacle_Destroyer_C|SetMovement_Speed _returnvalue (- (Variables|/Game/Blueprints/Obstacle_Destroyer.Obstacle_Destroyer_C|GetMovement_Speed _returnvalue) (Variables|Default|GetDestroyer_Movement_Speed)))
      (else
        (Variables|/Game/Blueprints/Obstacle_Destroyer.Obstacle_Destroyer_C|SetMovement_Speed _returnvalue (+ (Variables|/Game/Blueprints/Obstacle_Destroyer.Obstacle_Destroyer_C|GetMovement_Speed _returnvalue) (Variables|Default|GetDestroyer_Movement_Speed)))))
    (Variables|Default|SetDestroyer_Spawn_Delay 6e+01)
    (Variables|Default|SetDestroyer_Movement_Direction (not (Variables|Default|GetDestroyer_Movement_Direction)))
    (Variables|Default|SetSpawn%20Counter (+ (Variables|Default|GetSpawn%20Counter) 1.0))
    (if (Variables|Default|GetDestroyer_Movement_Direction)
      (Variables|Default|SetDestroyer_Spawn_Point 1.2e+03)
      (else
        (Variables|Default|SetDestroyer_Spawn_Point -4e+02)))
    (bind _returnvalue_2 (Game|SpawnActorfromClass "/Game/Blueprints/Obstacle_Destroyer.Obstacle_Destroyer_C" (Math|Transform|MakeTransform (Math|Vector|MakeVector (Variables|Default|GetDestroyer_Spawn_Point) 0.0 (Variables|Default|GetDestroyer_Spawn_Height)) "0, 0, 0" "1.000000,1,1") "Undefined" 0 0))
    (if (Variables|Default|GetDestroyer_Movement_Direction)
      (Variables|/Game/Blueprints/Obstacle_Destroyer.Obstacle_Destroyer_C|SetMovement_Speed _returnvalue_2 (- (Variables|/Game/Blueprints/Obstacle_Destroyer.Obstacle_Destroyer_C|GetMovement_Speed _returnvalue_2) (Variables|Default|GetDestroyer_Movement_Speed)))
      (else
        (Variables|/Game/Blueprints/Obstacle_Destroyer.Obstacle_Destroyer_C|SetMovement_Speed _returnvalue_2 (+ (Variables|/Game/Blueprints/Obstacle_Destroyer.Obstacle_Destroyer_C|GetMovement_Speed _returnvalue_2) (Variables|Default|GetDestroyer_Movement_Speed)))))
    (Variables|Default|SetDestroyer_Movement_Direction (not (Variables|Default|GetDestroyer_Movement_Direction)))
    (Variables|Default|SetSpawn%20Counter (+ (Variables|Default|GetSpawn%20Counter) 1.0))
    (else
      (Variables|Default|SetSpawn%20Counter 0.0))))

(fn ConstructionScript)