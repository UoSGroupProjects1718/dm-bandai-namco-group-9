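; Spawner actor that periodically creates pairs of Obstacle_Mine actors at a fixed X position and random heights.
; A Tick loop, gated by a Processing flag around a Delay, waits briefly before the first pair and longer between later ones.
; Each pair's mines receive opposite MovementSpeed offsets, with the direction order randomized once at BeginPlay.
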(event EventBeginPlay
  ;[1 1 1] Sets all values randomly upon loading in.
  (Variables|Default|SetMine_Movement_Direction (Math|Random|RandomBool))
  (Variables|Default|SetMine_Spawn_Height (Math|Random|RandomFloatinRange -3e+02 2e+01))
  (Variables|Default|SetMine_Movement_Speed 8e+01)
  (Variables|Default|SetMine_Spawn_Delay 5.0))

(event Collision|EventActorBeginOverlap
  (params (OtherActor :type Actor%20Object%20Reference)))

(event EventTick
  (params (DeltaSeconds :type Float%20%28single-precision%29))
  ;[1 1 1] First, checks if it's already proccessing a spawn. If not, it activates proccessing so it won't keep repeatedly spawning. After a (random) delay time, it spawns a seaweed clump at a randomly chosen height, and spawns it. It then gives it a speed value. If 'Seaweed Movement Direction' is true, it'll invert the speed, causing the seaweed to move the other way. It automatically switches direction each time it finishes spawning. Once it's done, processing is set back to false so the whole loop can start again.
  (if (not (Variables|Default|GetProcessing))
    (Variables|Default|SetProcessing true)
    (Utilities|FlowControl|Delay (Variables|Default|GetMine_Spawn_Delay))
    (bind _returnvalue (Game|SpawnActorfromClass "/Game/Blueprints/Obstacle_Mine.Obstacle_Mine_C" (Math|Transform|MakeTransform (Math|Vector|MakeVector 4e+02 1.0 (Variables|Default|GetMine_Spawn_Height))) "Undefined" 0 0))
    (if (Variables|Default|GetMine_Movement_Direction)
      (Variables|/Game/Blueprints/Obstacle_Mine.Obstacle_Mine_C|SetMovement%20Speed _returnvalue (- (Variables|/Game/Blueprints/Obstacle_Mine.Obstacle_Mine_C|GetMovement%20Speed _returnvalue) (Variables|Default|GetMine_Movement_Speed)))
      (else
        (Variables|/Game/Blueprints/Obstacle_Mine.Obstacle_Mine_C|SetMovement%20Speed _returnvalue (+ (Variables|/Game/Blueprints/Obstacle_Mine.Obstacle_Mine_C|GetMovement%20Speed _returnvalue) (Variables|Default|GetMine_Movement_Speed)))))
    (Variables|Default|SetMine_Spawn_Height (Math|Random|RandomFloatinRange -3e+02 2e+01))
    (Variables|Default|SetMine_Movement_Speed 8e+01)
    (Variables|Default|SetMine_Movement_Direction (not (Variables|Default|GetMine_Movement_Direction)))
    (bind _returnvalue_2 (Game|SpawnActorfromClass "/Game/Blueprints/Obstacle_Mine.Obstacle_Mine_C" (Math|Transform|MakeTransform (Math|Vector|MakeVector 4e+02 1.0 (Variables|Default|GetMine_Spawn_Height))) "Undefined" 0 0))
    (if (Variables|Default|GetMine_Movement_Direction)
      (Variables|/Game/Blueprints/Obstacle_Mine.Obstacle_Mine_C|SetMovement%20Speed _returnvalue_2 (- (Variables|/Game/Blueprints/Obstacle_Mine.Obstacle_Mine_C|GetMovement%20Speed _returnvalue_2) (Variables|Default|GetMine_Movement_Speed)))
      (else
        (Variables|/Game/Blueprints/Obstacle_Mine.Obstacle_Mine_C|SetMovement%20Speed _returnvalue_2 (+ (Variables|/Game/Blueprints/Obstacle_Mine.Obstacle_Mine_C|GetMovement%20Speed _returnvalue_2) (Variables|Default|GetMine_Movement_Speed)))))
    (Variables|Default|SetMine_Spawn_Height (Math|Random|RandomFloatinRange -3e+02 2e+01))
    (Variables|Default|SetMine_Movement_Speed 8e+01)
    (Variables|Default|SetMine_Spawn_Delay 15.0)
    (Variables|Default|SetMine_Movement_Direction (not (Variables|Default|GetMine_Movement_Direction)))
    (Variables|Default|SetProcessing false)))

(fn ConstructionScript)