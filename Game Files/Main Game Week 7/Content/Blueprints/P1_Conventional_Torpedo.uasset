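; Player 1's conventional torpedo, a projectile that travels along world X toward Player 2's submarines.
; Tick moves it by its current velocity, which rises by a fixed acceleration each frame until it reaches the maximum.
; Overlapping any listed P2 submarine class spawns an underwater explosion, then plays a hit sound and destroys the torpedo after a short delay.
; A timeout started at BeginPlay destroys torpedoes that miss.
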(event EventTick
  (params (DeltaSeconds :type Float%20%28single-precision%29))
  (bind _returnvalue (Transformation|GetActorLocation))
  (bind (_minimum_torpedo_velocity _torpedo_acceleration _maximum_torpedo_velocity) (|SpeedController))
  (bind (_x _y _z) (Math|Vector|BreakVector _returnvalue))
  ;[1 1 1] Causes the torpedo to automatically move. The torpedo will accelerate to a maxium value set by the relevant floats
  (Transformation|SetActorLocation (Math|Vector|MakeVector (+ _x (* (* (Variables|Default|GetMinimum_Torpedo_Velocity) 1.0) DeltaSeconds)) _y _z) false false)
  (if (< _minimum_torpedo_velocity _maximum_torpedo_velocity)
    (Variables|Default|SetMinimum_Torpedo_Velocity (+ _minimum_torpedo_velocity _torpedo_acceleration))))

(event EventBeginPlay
  ;[1 1 1] Auto-destroys the torpedo should it miss it's target.
  (Utilities|FlowControl|Delay 7.0)
  (Actor|DestroyActor)
  (Development|PrintString "Torpedo Timed out (P1)"))

(event Collision|EventActorBeginOverlap
  (params (OtherActor :type Actor%20Object%20Reference))
  (bind _returnvalue (Utilities|GetClass OtherActor))
  ;[1 1 1] Checks to see if the torpedo has hit it's target, then destroys it after a short delay to ensure it doesn't disapear before the hit was registered at the other end.
  (if (Math|Boolean|ORBoolean (Utilities|ClassIsChildOf _returnvalue "/Game/Blueprints/P2_Sub_JPN_Easy.P2_Sub_JPN_Easy_C") (Utilities|ClassIsChildOf _returnvalue "/Game/Blueprints/P2_Sub_JPN_Medium.P2_Sub_JPN_Medium_C") (Utilities|ClassIsChildOf _returnvalue "/Game/Blueprints/P2_Sub_JPN_Expert.P2_Sub_JPN_Expert_C") (Utilities|ClassIsChildOf _returnvalue "/Game/Blueprints/P2_Sub_RUS_Easy.P2_Sub_RUS_Easy_C") (Utilities|ClassIsChildOf _returnvalue "/Game/Blueprints/P2_Sub_RUS_Medium.P2_Sub_RUS_Medium_C") (Utilities|ClassIsChildOf _returnvalue "/Game/Blueprints/P2_Sub_RUS_Expert.P2_Sub_RUS_Expert_C") (Utilities|ClassIsChildOf _returnvalue "/Game/Blueprints/P2_Sub_TUR_Easy.P2_Sub_TUR_Easy_C") (Utilities|ClassIsChildOf _returnvalue "/Game/Blueprints/P2_Sub_TUR_Medium.P2_Sub_TUR_Medium_C") (Utilities|ClassIsChildOf _returnvalue "/Game/Blueprints/P2_Sub_TUR_Expert.P2_Sub_TUR_Expert_C"))
    (Development|PrintString "Hit confirmed, destroying torpedo (P1)")
    (Effects|SpawnEmitteratLocation "/Game/Particles/Underwater_Explosion.Underwater_Explosion" (Transformation|GetActorLocation))
    (Utilities|FlowControl|Delay 0.1)
    (Audio|SpawnSound2D "/Game/Audio/Torpedo_Hit.Torpedo_Hit")
    (Actor|DestroyActor)))

(fn ConstructionScript)